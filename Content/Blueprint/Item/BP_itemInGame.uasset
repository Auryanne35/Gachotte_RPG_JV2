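; BP_itemInGame is a world pickup actor that gives its item to the player when touched.
; On BeginPlay it sets its static mesh from the CurrentItem data.
; When a BP_TopDownCharacter overlaps its sphere, it passes the item and amount to the top-down controller, adds a small random number of seeds for that item, then destroys itself.
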(event `self.ReceiveBeginPlay`
  (`StaticMeshComponent.SetStaticMesh` (`self.StaticMesh`) (`/Game/Blueprint/Item/BlueprintData/BP_DA_Item.Mesh` (`self.currentItem`))))

(event `self.Sphere.OnComponentBeginOverlap`
  (params (OverlappedComponent :type "PrimitiveComponent Object Reference") (OtherActor :type "Actor Object Reference") (OtherComp :type "PrimitiveComponent Object Reference") (OtherBodyIndex :type Integer) (bFromSweep :type Boolean) (SweepResult :type "HitResult Structure (by ref)"))
  (bind _playercontroller (`/Game/Blueprint/BP_FL_shortcut.getTopDownController`))
  (bind _currentitem (`self.currentItem`))
  (cast `/Game/Base_Unreal/TopDown/Blueprints/BP_TopDownCharacter` OtherActor)
  (`/Game/Base_Unreal/TopDown/Blueprints/BP_TopDownController.addItem` _playercontroller _currentitem (`self.amount`))
  (`/Game/Base_Unreal/TopDown/Blueprints/BP_TopDownController.addSeed` _playercontroller _currentitem (`KismetMathLibrary.RandomIntegerInRange` 1 3))
  (`self.K2_DestroyActor`))

(fn `UserConstructionScript`)