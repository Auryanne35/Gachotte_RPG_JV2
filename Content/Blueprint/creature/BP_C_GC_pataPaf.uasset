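; Creature Blueprint for pataPaf, a tameable creature with its own health, reward and tame chance.
; It only overrides SetStartVariables to fill in those starting stats, with max HP copied from HP and tame chance at full.
; Its event graph holds only disabled stub events and its construction script just calls the parent, so all behavior is left to the parent class.
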(fn `setStartVariables`
  (bind _output_get (set `self.HP` 40))
  (set `self.HPMax` _output_get)
  (set `self.reward` 5)
  (set `self.tameChance` 1.0))

(fn `UserConstructionScript`
  (`parent.UserConstructionScript`))