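; BP_C_evilCreature is an AI-controlled enemy creature that detects the top-down player character and can be killed by damage.
; Its Sphere overlap passes the player to BP_AI_Controller through SetPlayer when the character enters, and clears that reference when it leaves.
; TakeDamage hands the amount to LoseLife and destroys the actor once HP reaches zero or below.
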(event `self.Sphere.OnComponentBeginOverlap`
  (params (OverlappedComponent :type "PrimitiveComponent Object Reference") (OtherActor :type "Actor Object Reference") (OtherComp :type "PrimitiveComponent Object Reference") (OtherBodyIndex :type Integer) (bFromSweep :type Boolean) (SweepResult :type "HitResult Structure (by ref)"))
  (bind _asbp_top_down_character (cast `/Game/Base_Unreal/TopDown/Blueprints/BP_TopDownCharacter` OtherActor))
  (bind _asbp_ai_controller (cast `/Game/Blueprint/BP_AI_Controller` (`self.GetController`)))
  (`/Game/Blueprint/BP_AI_Controller.SetPlayer` _asbp_ai_controller _asbp_top_down_character))

(event `self.Sphere.OnComponentEndOverlap`
  (params (OverlappedComponent :type "PrimitiveComponent Object Reference") (OtherActor :type "Actor Object Reference") (OtherComp :type "PrimitiveComponent Object Reference") (OtherBodyIndex :type Integer))
  (cast `/Game/Base_Unreal/TopDown/Blueprints/BP_TopDownCharacter` OtherActor)
  (bind _asbp_ai_controller (cast `/Game/Blueprint/BP_AI_Controller` (`self.GetController`)))
  (`/Game/Blueprint/BP_AI_Controller.SetPlayer` _asbp_ai_controller null))

(fn `takeDamage`
  (params (NewParam :type Integer))
  (`self.loseLife` NewParam)
  (if (<= (`self.HP`) 0)
    (`self.K2_DestroyActor`)))

(fn `UserConstructionScript`
  (`parent.UserConstructionScript`))