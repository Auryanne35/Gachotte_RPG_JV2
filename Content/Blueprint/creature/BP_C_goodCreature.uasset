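; BP_C_goodCreature is a child creature Blueprint for a tameable creature that wanders, takes damage and can be teleported to an enclosure.
; It loops AI moves to random nearby reachable points, pausing randomly between them.
; When Tameable, damage lowers HP and raises the tame chance, shown on camera-facing text.
; At zero HP it pays a money reward, refreshes the inventory UI and destroys itself.
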(event `self.ReceiveBeginPlay`
  (`parent.ReceiveBeginPlay`)
  (`TextRenderComponent.K2_SetText` (`self.TextRender1`) (`KismetTextLibrary.Conv_IntToText` (`KismetMathLibrary.FTrunc` (`self.tameChance`))))
  (`self.getLocation`))

(event `self.ReceiveTick`
  (params (DeltaSeconds :type "Float (single-precision)"))
  (`parent.ReceiveTick` DeltaSeconds)
  (`SceneComponent.K2_SetWorldRotation` (`self.TextRender1`) (`KismetMathLibrary.FindLookAtRotation` (`SceneComponent.K2_GetComponentLocation` (`self.TextRender1`)) (`PlayerCameraManager.GetCameraLocation` (`PlayerController.PlayerCameraManager` (`/Game/Blueprint/BP_FL_shortcut.getTopDownController`)))) false false))

(event `getLocation`
  (set `self.Random Location` (`NavigationSystemV1.K2_GetRandomReachablePointInRadius` (`self.K2_GetActorLocation`) 1000.0 null null))
  (`self.goToLocation`))

(event `goToLocation`
  (`|AIMoveTo` self (`self.Random Location`) null
    (:`OnSuccess`
      _)
    (:`OnFail`
      _))
  (`KismetSystemLibrary.Delay` (`KismetMathLibrary.RandomFloatInRange` 2.0 5.0))
  (`self.getLocation`))

(fn `changeTameChance`
  (bind _output_get (set `self.tameChance` (* (- 1.0 (/ (`self.HP`) (`self.HPMax`))) 100.0)))
  (`TextRenderComponent.K2_SetText` (`self.TextRender1`) (`KismetTextLibrary.Conv_IntToText` (`KismetMathLibrary.FTrunc` _output_get))))

(fn `setTextLife`
  (`parent.setTextLife`))

(fn `takeDamage`
  (params (NewParam :type Integer))
  (bind _playercontroller (`/Game/Blueprint/BP_FL_shortcut.getTopDownController`))
  (if (`self.tameable`)
    (`self.loseLife` NewParam)
    (`self.changeTameChance`)
    (if (<= (`self.HP`) 0)
      (set `/Game/Base_Unreal/TopDown/Blueprints/BP_TopDownController.Money` (+ (`/Game/Base_Unreal/TopDown/Blueprints/BP_TopDownController.Money` _playercontroller) (`self.reward`)) _playercontroller)
      (`/Game/UI/WBP_inventory.updateUI` (`/Game/Base_Unreal/TopDown/Blueprints/BP_TopDownController.UIInventory` _playercontroller))
      (`self.K2_DestroyActor`))))

(fn `teleportToEnclosure`
  (`self.K2_SetActorRelativeLocation` (`self.K2_GetActorLocation` (`self.enclosureToTeleport`))))

(fn `UserConstructionScript`
  (`parent.UserConstructionScript`))