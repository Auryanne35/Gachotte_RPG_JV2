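; BP_creature is a creature Blueprint that tracks HP and shows it on a floating text label with a "pv" suffix.
; BeginPlay calls SetStartVariables and refreshes the label, and LoseLife subtracts an amount from HP before refreshing it again.
; Every Tick, the label rotates to face the top-down controller's camera.
; SetStartVariables and TakeDamage are empty here, so LoseLife is not called within this graph.
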(event `self.ReceiveBeginPlay`
  (`self.setStartVariables`)
  (`self.setTextLife`))

(event `self.ReceiveTick`
  (params (DeltaSeconds :type "Float (single-precision)"))
  (`SceneComponent.K2_SetWorldRotation` (`self.TextRender`) (`KismetMathLibrary.FindLookAtRotation` (`SceneComponent.K2_GetComponentLocation` (`self.TextRender`)) (`PlayerCameraManager.GetCameraLocation` (`PlayerController.PlayerCameraManager` (`/Game/Blueprint/BP_FL_shortcut.getTopDownController`)))) false false))

(fn `loseLife`
  (params (Amount :type Integer))
  (set `self.HP` (- (`self.HP`) Amount))
  (`self.setTextLife`))

(fn `setStartVariables`)

(fn `setTextLife`
  (`TextRenderComponent.K2_SetText` (`self.TextRender`) (`KismetTextLibrary.Conv_StringToText` (`KismetStringLibrary.Concat_StrStr` (`KismetStringLibrary.Conv_IntToString` (`self.HP`)) " pv"))))

(fn `takeDamage`
  (params (NewParam :type Integer)))

(fn `UserConstructionScript`)