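; BP_evilCreature is an enemy creature with hit points and a floating health label.
; A sphere overlap passes the top-down character to its BP_AI_Controller as the player reference and clears it when the character leaves.
; LoseLife subtracts from HP and refreshes the "pv" text, which turns toward the camera every tick.
; SetStartVariables runs at BeginPlay but is empty here.
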(event `self.ReceiveBeginPlay`
  (`self.setStartVariables`)
  (`self.setTextLife`))

(event `self.ReceiveTick`
  (params (DeltaSeconds :type "Float (single-precision)"))
  (`SceneComponent.K2_SetWorldRotation` (`self.TextRender`) (`KismetMathLibrary.FindLookAtRotation` (`SceneComponent.K2_GetComponentLocation` (`self.TextRender`)) (`PlayerCameraManager.GetCameraLocation` (`PlayerController.PlayerCameraManager` (`/Game/Blueprint/BP_FL_shortcut.getTopDownController`)))) false false))

(event `self.Sphere.OnComponentBeginOverlap`
  (params (OverlappedComponent :type "PrimitiveComponent Object Reference") (OtherActor :type "Actor Object Reference") (OtherComp :type "PrimitiveComponent Object Reference") (OtherBodyIndex :type Integer) (bFromSweep :type Boolean) (SweepResult :type "HitResult Structure (by ref)"))
  (bind _asbp_top_down_character (cast `/Game/Base_Unreal/TopDown/Blueprints/BP_TopDownCharacter` OtherActor))
  (bind _asbp_ai_controller (cast `/Game/Blueprint/BP_AI_Controller` (`self.GetController`)))
  (`/Game/Blueprint/BP_AI_Controller.SetPlayer` _asbp_ai_controller _asbp_top_down_character))

(event `self.Sphere.OnComponentEndOverlap`
  (params (OverlappedComponent :type "PrimitiveComponent Object Reference") (OtherActor :type "Actor Object Reference") (OtherComp :type "PrimitiveComponent Object Reference") (OtherBodyIndex :type Integer))
  (cast `/Game/Base_Unreal/TopDown/Blueprints/BP_TopDownCharacter` OtherActor)
  (bind _asbp_ai_controller (cast `/Game/Blueprint/BP_AI_Controller` (`self.GetController`)))
  (`/Game/Blueprint/BP_AI_Controller.SetPlayer` _asbp_ai_controller null))

(fn `loseLife`
  (params (Amount :type Integer))
  (set `self.HP` (- (`self.HP`) Amount))
  (`self.setTextLife`))

(fn `setStartVariables`)

(fn `setTextLife`
  (`TextRenderComponent.K2_SetText` (`self.TextRender`) (`KismetTextLibrary.Conv_StringToText` (`KismetStringLibrary.Concat_StrStr` (`KismetTextLibrary.Conv_TextToString` (`KismetTextLibrary.Conv_IntToText` (`self.HP`))) " pv"))))

(fn `UserConstructionScript`)