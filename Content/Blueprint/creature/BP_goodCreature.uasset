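; BP_goodCreature is a wandering creature that shows its HP as floating "pv" text.
; An AIMoveTo loop sends it to random reachable nearby points, pausing briefly after each success or failure.
; takeDamage sweeps it toward a relative location derived from the Arrow's reversed forward vector, not offset from its position, then calls LoseLife with zero damage.
; LoseLife updates HP and text, destroying the actor at zero or below.
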(event `self.ReceiveBeginPlay`
  (`self.getLocation`)
  (`self.setTextLife`))

(event `getLocation`
  (set `self.Random Location` (`NavigationSystemV1.K2_GetRandomReachablePointInRadius` (`self.K2_GetActorLocation`) 1000.0 null null))
  (`self.goToLocation`))

(event `goToLocation`
  (`|AIMoveTo` self (`self.Random Location`) null
    (:`OnSuccess`
      _)
    (:`OnFail`
      _))
  (`KismetSystemLibrary.Delay` (`KismetMathLibrary.RandomFloatInRange` 2.0 5.0))
  (`self.getLocation`))

(event `takeDamage`
  (`self.K2_SetActorRelativeLocation` (* (`SceneComponent.GetForwardVector` (`self.Arrow1`)) -10000) true)
  (`self.loseLife` 0))

(fn `loseLife`
  (params (NewParam :type Integer))
  (set `self.HP` (- (`self.HP`) NewParam))
  (`self.setTextLife`)
  (if (<= (`self.HP`) 0)
    (`self.K2_DestroyActor`)))

(fn `setTextLife`
  (`TextRenderComponent.K2_SetText` (`self.TextRender`) (`KismetTextLibrary.Conv_StringToText` (`KismetStringLibrary.Concat_StrStr` (`KismetTextLibrary.Conv_TextToString` (`KismetTextLibrary.Conv_IntToText` (`self.HP`))) " pv"))))

(fn `UserConstructionScript`)