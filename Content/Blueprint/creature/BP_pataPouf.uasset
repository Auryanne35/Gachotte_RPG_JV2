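; BP_pataPouf is a creature that wanders the level on its own from BeginPlay.
; It picks a random reachable navigation point within a fixed radius of its current position and walks there with AI MoveTo.
; On success or failure, it waits a short random delay before picking a new point, forming an endless event-driven loop without Tick.
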(event `self.ReceiveBeginPlay`
  (`self.get location`))

(event `get location`
  (set `self.Random Location` (`NavigationSystemV1.K2_GetRandomReachablePointInRadius` (`self.K2_GetActorLocation`) 1000.0 null null))
  (`self.goToLocation`))

(event `goToLocation`
  (`|AIMoveTo` self (`self.Random Location`) null
    (:`OnSuccess`
      _)
    (:`OnFail`
      _))
  (`KismetSystemLibrary.Delay` (`KismetMathLibrary.RandomFloatInRange` 2.0 5.0))
  (`self.get location`))

(fn `UserConstructionScript`)