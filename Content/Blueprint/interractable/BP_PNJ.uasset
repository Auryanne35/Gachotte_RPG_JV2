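; BP_PNJ is an interactable NPC that toggles a dialogue view each time its Interract event fires.
; A FlipFlop first blends the top-down camera to the NPC, disables player movement, hides one text render and shows another.
; That text is picked by NumQuest: default text, or Quest.TextStart for cases 0-3, though each assigns Quest to None first.
; The next interaction restores the pawn camera, movement and original text visibility.
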(event `self.interract`
  (bind _playercontroller (`/Game/Blueprint/BP_FL_shortcut.getTopDownController`))
  (bind _playercontroller_2 (`/Game/Blueprint/BP_FL_shortcut.getTopDownController`))
  (`/Engine/EditorBlueprintResources/StandardMacros.FlipFlop`
    (:`A`
      (`PlayerController.SetViewTargetWithBlend` _playercontroller_2 self 0.5 "VTBlend_Linear" 0.0 false)
      (set `/Game/Base_Unreal/TopDown/Blueprints/BP_TopDownController.move` false _playercontroller_2)
      (`SceneComponent.SetHiddenInGame` (`self.TextRender`) true false)
      (`SceneComponent.SetVisibility` (`self.TextRender1`) true false)
      (switch `int` (`self.numQuest`)
        (:`Default`
          (`TextRenderComponent.K2_SetText` (`self.TextRender1`) (`self.textDefault`)))
        (:`0`
          (bind _output_get (set `self.quest` null))
          (`TextRenderComponent.K2_SetText` (`self.TextRender1`) (`/Game/Blueprint/Item/BlueprintData/BP_DA_Quest.textStart` _output_get)))
        (:`1`
          (bind _output_get_2 (set `self.quest` null))
          (`TextRenderComponent.K2_SetText` (`self.TextRender1`) (`/Game/Blueprint/Item/BlueprintData/BP_DA_Quest.textStart` _output_get_2)))
        (:`2`
          (bind _output_get_3 (set `self.quest` null))
          (`TextRenderComponent.K2_SetText` (`self.TextRender1`) (`/Game/Blueprint/Item/BlueprintData/BP_DA_Quest.textStart` _output_get_3)))
        (:`3`
          (bind _output_get_4 (set `self.quest` null))
          (`TextRenderComponent.K2_SetText` (`self.TextRender1`) (`/Game/Blueprint/Item/BlueprintData/BP_DA_Quest.textStart` _output_get_4)))))
    (:`B`
      (`SceneComponent.SetVisibility` (`self.TextRender1`) false false)
      (`PlayerController.SetViewTargetWithBlend` _playercontroller (`Controller.K2_GetPawn` _playercontroller) 0.5 "VTBlend_Linear" 0.0 false)
      (set `/Game/Base_Unreal/TopDown/Blueprints/BP_TopDownController.move` true _playercontroller)
      (`SceneComponent.SetHiddenInGame` (`self.TextRender`) false false))))

(fn `UserConstructionScript`
  (`parent.UserConstructionScript`))