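; BP_campfire is an interactable campfire that opens a cooking screen when used.
; Each interaction toggles via a FlipFlop between cooking and normal play.
; Entering blends the camera to the campfire, disables top-down controller movement, hides the prompt text and shows the WBP_cooking widget, initialized with this campfire.
; Leaving blends the view back to the controlled pawn, restores movement and text, and hides the widget.
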(event `self.interract`
  (bind _playercontroller (`/Game/Blueprint/BP_FL_shortcut.getTopDownController`))
  (bind _playercontroller_2 (`/Game/Blueprint/BP_FL_shortcut.getTopDownController`))
  (bind _widget (`self.Widget`))
  (`/Engine/EditorBlueprintResources/StandardMacros.FlipFlop`
    (:`A`
      (`PlayerController.SetViewTargetWithBlend` _playercontroller_2 self 0.5 "VTBlend_Linear" 0.0 false)
      (set `/Game/Base_Unreal/TopDown/Blueprints/BP_TopDownController.move` false _playercontroller_2)
      (`SceneComponent.SetHiddenInGame` (`self.TextRender`) true false)
      (`SceneComponent.SetVisibility` _widget true false)
      (bind _aswbp_cooking (cast `/Game/UI/WBP_cooking` (`WidgetComponent.GetWidget` _widget)))
      (`/Game/UI/WBP_cooking.initializeCamp` _aswbp_cooking self))
    (:`B`
      (`PlayerController.SetViewTargetWithBlend` _playercontroller (`Controller.K2_GetPawn` _playercontroller) 0.5 "VTBlend_Linear" 0.0 false)
      (set `/Game/Base_Unreal/TopDown/Blueprints/BP_TopDownController.move` true _playercontroller)
      (`SceneComponent.SetHiddenInGame` (`self.TextRender`) false false)
      (`SceneComponent.SetVisibility` (`self.Widget`) false false))))

(fn `UserConstructionScript`
  (`parent.UserConstructionScript`))