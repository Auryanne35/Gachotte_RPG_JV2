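; Interactable crop field where the player plants seeds, waits for them to grow and harvests the yield.
; Interacting while idle toggles a camera blend to the field and its WBP_field widget, pausing player movement.
; fieldBusy spends four seeds from the controller, closes the menu and waits the item's grow time before setting the crop mesh.
; Interacting with a grown crop adds the harvest to the controller and hides the mesh.
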(event `self.interract`
  (bind _playercontroller (`/Game/Blueprint/BP_FL_shortcut.getTopDownController`))
  (bind _playercontroller_2 (`/Game/Blueprint/BP_FL_shortcut.getTopDownController`))
  (bind _widget (`self.Widget`))
  (if (`self.itGrows`)
    _
    (elif (`self.itsGood`)
      (`/Game/Base_Unreal/TopDown/Blueprints/BP_TopDownController.addItem` (`/Game/Blueprint/BP_FL_shortcut.getTopDownController`) (`/Game/Blueprint/Item/BlueprintData/BP_DA_Seed.recolt` (`self.recolt`)) 5)
      (set `self.itsGood` false)
      (`SceneComponent.SetVisibility` (`self.StaticMesh`) false false)
      (else
        (`/Engine/EditorBlueprintResources/StandardMacros.FlipFlop`
          (:`A`
            (`PlayerController.SetViewTargetWithBlend` _playercontroller_2 self 0.5 "VTBlend_Linear" 0.0 false)
            (set `/Game/Base_Unreal/TopDown/Blueprints/BP_TopDownController.move` false _playercontroller_2)
            (`SceneComponent.SetHiddenInGame` (`self.TextRender`) true false)
            (`SceneComponent.SetVisibility` _widget true false)
            (bind _aswbp_field (cast `/Game/UI/WBP_field` (`WidgetComponent.GetWidget` _widget)))
            (`/Game/UI/WBP_field.initializeField` _aswbp_field self))
          (:`B`
            (`PlayerController.SetViewTargetWithBlend` _playercontroller (`Controller.K2_GetPawn` _playercontroller) 0.5 "VTBlend_Linear" 0.0 false)
            (set `/Game/Base_Unreal/TopDown/Blueprints/BP_TopDownController.move` true _playercontroller)
            (`SceneComponent.SetHiddenInGame` (`self.TextRender`) false false)
            (`SceneComponent.SetVisibility` (`self.Widget`) false false)))))))

(event `fieldBusy`
  (params (itemToPlant :type "/Game/Blueprint/Item/BlueprintData/BP_DA_Seed Object Reference (by ref)"))
  (bind _playercontroller (`/Game/Blueprint/BP_FL_shortcut.getTopDownController`))
  (bind _seeds (`/Game/Base_Unreal/TopDown/Blueprints/BP_TopDownController.seeds` (`/Game/Blueprint/BP_FL_shortcut.getTopDownController`)))
  (bind _value (`BlueprintMapLibrary.Map_Find` _seeds itemToPlant))
  (if (`BlueprintMapLibrary.Map_Contains` _seeds itemToPlant)
    (if (>= _value 4)
      (`BlueprintMapLibrary.Map_Add` _seeds itemToPlant (- _value 4))
      (set `self.futureField` (`/Game/Blueprint/Item/BlueprintData/BP_DA_Seed.meshField` itemToPlant))
      (`SceneComponent.SetVisibility` (`self.StaticMesh`) true false)
      (bind _returnvalue (`AddComponent|NODE_AddStaticMeshComponent-5`))
      (set `self.StaticMesh` _returnvalue)
      (set `self.itGrows` true)
      (`PlayerController.SetViewTargetWithBlend` _playercontroller (`Controller.K2_GetPawn` _playercontroller) 0.5 "VTBlend_Linear" 0.0 false)
      (set `/Game/Base_Unreal/TopDown/Blueprints/BP_TopDownController.move` true _playercontroller)
      (`SceneComponent.SetHiddenInGame` (`self.TextRender`) false false)
      (`SceneComponent.SetVisibility` (`self.Widget`) false false)
      (set `self.recolt` itemToPlant)
      (`KismetSystemLibrary.PrintString` "Hello")
      (`KismetSystemLibrary.Delay` (`KismetMathLibrary.Conv_IntToDouble` (`/Game/Blueprint/Item/BlueprintData/BP_DA_Seed.growTime` itemToPlant)))
      (set `self.itGrows` false)
      (set `self.itsGood` true)
      (`StaticMeshComponent.SetStaticMesh` (`self.StaticMesh`) (`/Game/Blueprint/Item/BlueprintData/BP_DA_Seed.meshField` itemToPlant)))))

(fn `UserConstructionScript`
  (`parent.UserConstructionScript`))