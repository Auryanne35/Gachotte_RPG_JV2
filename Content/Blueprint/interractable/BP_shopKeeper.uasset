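; BP_shopKeeper is an interactable shopkeeper actor that opens and closes a shop UI when the player interacts with it.
; A FlipFlop on Interract alternates between opening and closing.
; Opening blends the camera to the shopkeeper, shows the WBP_shop widget, initializes it with this actor, disables movement via the TopDown controller and swaps the text renders.
; Closing returns the view to the pawn and restores movement and visibility.
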(event `self.interract`
  (bind _playercontroller (`/Game/Blueprint/BP_FL_shortcut.getTopDownController`))
  (bind _playercontroller_2 (`/Game/Blueprint/BP_FL_shortcut.getTopDownController`))
  (bind _widget (`self.Widget`))
  (`/Engine/EditorBlueprintResources/StandardMacros.FlipFlop`
    (:`A`
      (`SceneComponent.SetVisibility` (`self.TextRender1`) true false)
      (`PlayerController.SetViewTargetWithBlend` _playercontroller_2 self 0.5 "VTBlend_Linear" 0.0 false)
      (`SceneComponent.SetVisibility` _widget true false)
      (bind _aswbp_shop (cast `/Game/UI/WBP_shop` (`WidgetComponent.GetWidget` _widget)))
      (`/Game/UI/WBP_shop.initializeShop` _aswbp_shop self)
      (set `/Game/Base_Unreal/TopDown/Blueprints/BP_TopDownController.move` false _playercontroller_2)
      (`SceneComponent.SetHiddenInGame` (`self.TextRender`) true false))
    (:`B`
      (`SceneComponent.SetVisibility` (`self.TextRender1`) false false)
      (`PlayerController.SetViewTargetWithBlend` _playercontroller (`Controller.K2_GetPawn` _playercontroller) 0.5 "VTBlend_Linear" 0.0 false)
      (set `/Game/Base_Unreal/TopDown/Blueprints/BP_TopDownController.move` true _playercontroller)
      (`SceneComponent.SetHiddenInGame` (`self.TextRender`) false false)
      (`SceneComponent.SetVisibility` (`self.Widget`) false false))))

(fn `UserConstructionScript`
  (`parent.UserConstructionScript`))