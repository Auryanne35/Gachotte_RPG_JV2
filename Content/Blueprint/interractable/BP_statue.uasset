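; BP_statue is an interactable statue that restores the player's HP and FarmPoint to their maximums.
; Interract alternates through a FlipFlop between entering and leaving a focused view.
; Entering blends the camera to the statue, disables movement on the top-down controller, swaps the visible text renders, refills both stats and updates the inventory UI.
; Leaving returns the camera to the controlled pawn, re-enables movement and restores the texts.
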(event `self.interract`
  (bind _playercontroller (`/Game/Blueprint/BP_FL_shortcut.getTopDownController`))
  (bind _playercontroller_2 (`/Game/Blueprint/BP_FL_shortcut.getTopDownController`))
  (bind _playercontroller_3 (`/Game/Blueprint/BP_FL_shortcut.getTopDownController`))
  (`/Engine/EditorBlueprintResources/StandardMacros.FlipFlop`
    (:`A`
      (`SceneComponent.SetVisibility` (`self.TextRender1`) true false)
      (`PlayerController.SetViewTargetWithBlend` _playercontroller_3 self 0.5 "VTBlend_Linear" 0.0 false)
      (set `/Game/Base_Unreal/TopDown/Blueprints/BP_TopDownController.move` false _playercontroller_3)
      (`SceneComponent.SetHiddenInGame` (`self.TextRender`) true false)
      (set `/Game/Base_Unreal/TopDown/Blueprints/BP_TopDownController.HP` (`/Game/Base_Unreal/TopDown/Blueprints/BP_TopDownController.HPMax` _playercontroller_2) _playercontroller_2)
      (set `/Game/Base_Unreal/TopDown/Blueprints/BP_TopDownController.farmPoint` (`/Game/Base_Unreal/TopDown/Blueprints/BP_TopDownController.maxFarmPoint` _playercontroller_2) _playercontroller_2)
      (`/Game/UI/WBP_inventory.updateUI` (`/Game/Base_Unreal/TopDown/Blueprints/BP_TopDownController.UIInventory` _playercontroller_2)))
    (:`B`
      (`SceneComponent.SetVisibility` (`self.TextRender1`) false false)
      (`PlayerController.SetViewTargetWithBlend` _playercontroller (`Controller.K2_GetPawn` _playercontroller) 0.5 "VTBlend_Linear" 0.0 false)
      (set `/Game/Base_Unreal/TopDown/Blueprints/BP_TopDownController.move` true _playercontroller)
      (`SceneComponent.SetHiddenInGame` (`self.TextRender`) false false))))

(fn `UserConstructionScript`
  (`parent.UserConstructionScript`))