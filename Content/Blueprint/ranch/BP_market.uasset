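; BP_market is a market actor for the ranch that shows its name on a floating text label.
; On BeginPlay it sets the TextRender text from the NameMarket variable.
; Every Tick it rotates the label to face the top-down player controller's camera, billboard style.
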(event `self.ReceiveBeginPlay`
  (`TextRenderComponent.K2_SetText` (`self.TextRender`) (`self.nameMarket`)))

(event `self.ReceiveTick`
  (params (DeltaSeconds :type "Float (single-precision)"))
  (`SceneComponent.K2_SetWorldRotation` (`self.TextRender`) (`KismetMathLibrary.FindLookAtRotation` (`SceneComponent.K2_GetComponentLocation` (`self.TextRender`)) (`PlayerCameraManager.GetCameraLocation` (`PlayerController.PlayerCameraManager` (`/Game/Blueprint/BP_FL_shortcut.getTopDownController`)))) false false))

(fn `UserConstructionScript`)